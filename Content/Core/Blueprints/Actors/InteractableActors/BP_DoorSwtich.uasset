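; BP_DoorSwtich is a door that slides vertically once enough switches are active.
; SwitchActivated and SwitchDeactivated adjust an active count, then play or reverse the door timeline depending on whether it reaches SwitchesNeeded.
; The timeline lerps the actor between its start location and an end height derived from its bounds at BeginPlay.
; Timeline event tracks trigger open and close sounds, each gated on the switch count to match the travel direction.
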(event `self.ReceiveBeginPlay`
  (bind (_origin _boxextent) (`self.GetActorBounds` false true))
  (bind _output_get (set `self.StartLocation` (`self.K2_GetActorLocation`)))
  (bind _result (`/Engine/EditorBlueprintResources/StandardMacros.NegateFloat` (- (+ (.z _origin) (.z _boxextent)) 213.0))
    (:`  `
      (set `self.EndLocation` (`KismetMathLibrary.MakeVector` (.x _output_get) (.y _output_get) _result)))))

(event `SwitchActivated`
  (bind _tm_door (`self.TM_door`))
  (`/Engine/EditorBlueprintResources/StandardMacros.IncrementInt` (`self.SwtichesActive`)
    (:`  `
      (if (>= (`self.SwtichesActive`) (`self.SwitchesNeeded`))
        (`TimelineComponent.Play` _tm_door :!label _label)
        (else
          (`TimelineComponent.Reverse` _tm_door :!label _label_2))))))

(event `SwitchDeactivated`
  (set `self.SwtichesActive` (`KismetMathLibrary.Clamp` (- (`self.SwtichesActive`) 1) 0 (`self.SwitchesNeeded`)))
  (if (>= (`self.SwtichesActive`) (`self.SwitchesNeeded`))
    (goto _label)
    (else
      (goto _label_2))))

(fn `PlayCloseSound`
  (if (not (>= (`self.SwtichesActive`) (`self.SwitchesNeeded`)))
    (`GameplayStatics.PlaySoundAtLocation` "/Engine/EditorSounds/GamePreview/EjectFromPlayer.EjectFromPlayer" (`self.K2_GetActorLocation`) (struct) 1.0 1.0 0.0 null null null null)))

(fn `PlayOpenSound`
  (if (>= (`self.SwtichesActive`) (`self.SwitchesNeeded`))
    (`GameplayStatics.PlaySoundAtLocation` "/Engine/EditorSounds/GamePreview/EndPlayInEditor.EndPlayInEditor" (`self.K2_GetActorLocation`) (struct) 1.0 1.0 0.0 null null null null)))

(fn `UserConstructionScript`)