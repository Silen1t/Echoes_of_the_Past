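; BP_InventoryItemComponent is an actor component that holds the inventory data for an item: type, name, icon, description and ID.
; On BeginPlay, Note items take their name from the note title and build their description from the note's location and content.
; Getter and setter functions expose the data.
; SetKeyID generates a random ID and shares it with the assigned DoorKeyActor and the item's info, linking key to door.
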(event `self.ReceiveBeginPlay`
  (bind (_noteinfo_title _noteinfo_location _noteinfo_content) (break `/Game/Core/Blueprints/Structures/FNote` (`self.NoteInfo`)))
  (bind (_iteminfo_itemtype _iteminfo_name _iteminfo_icon _iteminfo_description _iteminfo_id) (break `/Game/Core/Blueprints/Structures/FItemInfo` (`self.ItemInfo`)))
  (switch `/Game/Core/Blueprints/Enumeration/EItemType` _iteminfo_itemtype
    (:`NewEnumerator1`
      (set `self.ItemInfo` (make `/Game/Core/Blueprints/Structures/FItemInfo` _iteminfo_itemtype _noteinfo_title _iteminfo_icon (`KismetTextLibrary.Conv_TextToString` (`|FormatText` "Location:{Location info} \n \n \n{Content}" _noteinfo_location _noteinfo_content)) _iteminfo_id)))))

(fn `GetItemInfo`
  (returns (ItemInfo :type "/Game/Core/Blueprints/Structures/FItemInfo Structure"))
  (return (`self.ItemInfo`)))

(fn `SetDoorKeyActor`
  (params (DoorKeyActor :type "/Game/Core/Blueprints/Actors/InteractableActors/BP_DoorKey Object Reference"))
  (set `self.DoorKeyActor` DoorKeyActor))

(fn `SetItemInfo`
  (params (ItemInfo :type "/Game/Core/Blueprints/Structures/FItemInfo Structure"))
  (set `self.ItemInfo` ItemInfo))

(fn `SetKeyID`
  (locals (ID :type Integer))
  (bind (_iteminfo_itemtype _iteminfo_name _iteminfo_icon _iteminfo_description) (break `/Game/Core/Blueprints/Structures/FItemInfo` (`self.ItemInfo`)))
  (set `local.ID` (`KismetMathLibrary.RandomInteger` 100000))
  (`/Game/Core/Blueprints/Actors/InteractableActors/BP_DoorKey.SetDoorKeyID` (`self.DoorKeyActor`) (`local.ID`))
  (`self.SetItemInfo` (make `/Game/Core/Blueprints/Structures/FItemInfo` _iteminfo_itemtype _iteminfo_name _iteminfo_icon _iteminfo_description (`local.ID`))))