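; Test pickup actor that the player interacts with to add an item to their inventory.
; An inventory item component holds the item info, and on BeginPlay Key-type items are given their door key actor and have their key ID set.
; The interactable component's interact event passes the item info to the interacting player, then the actor destroys itself.
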(event `self.ReceiveBeginPlay`
  (bind _iteminfo_itemtype (break `/Game/Core/Blueprints/Structures/FItemInfo` (`/Game/Core/Blueprints/Components/BP_InventoryItemComponent.GetItemInfo` (`self.BP_InventoryItemComponent`))))
  (switch `/Game/Core/Blueprints/Enumeration/EItemType` _iteminfo_itemtype
    (:`NewEnumerator0`
      (`/Game/Core/Blueprints/Components/BP_InventoryItemComponent.SetDoorKeyActor` (`self.BP_InventoryItemComponent`) (`self.BP_DoorKey`))
      (`/Game/Core/Blueprints/Components/BP_InventoryItemComponent.SetKeyID` (`self.BP_InventoryItemComponent`)))))

(event `self.BP_InteractableComponent.OnObjectInteract`
  (params (Player :type "/Game/Core/Blueprints/Characters/FirstPerson/BP_FirstPersonCharacter Object Reference"))
  (`/Game/Core/Blueprints/Characters/FirstPerson/BP_FirstPersonCharacter.AddInventoryItem` Player (`/Game/Core/Blueprints/Components/BP_InventoryItemComponent.GetItemInfo` (`self.BP_InventoryItemComponent`)))
  (`self.K2_DestroyActor`))

(fn `UserConstructionScript`)