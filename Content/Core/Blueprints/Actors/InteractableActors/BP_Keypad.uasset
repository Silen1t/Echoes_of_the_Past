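; Interactable keypad actor that opens a linked door when the player enters the correct numeric password.
; Child-actor buttons receive a keypad reference on BeginPlay, and digits build a capped array shown on a text render component.
; A wrong code plays a sound and lights the red emissive dynamic material.
; A correct code lights the green one, activates DoorActor and removes the buttons' interactable components to lock the keypad.
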(event `self.ReceiveBeginPlay`
  (`self.InitializeKeypadButtons`))

(event `InitializeKeypadButtons`
  (for _array_element (`self.GetKeypadButtonArray`)
    (bind _returnvalue (`self.GetComponentByClass` (`ChildActorComponent.ChildActor` _array_element) "/Game/Core/Blueprints/Components/BP_KeypadButtonComponent.BP_KeypadButtonComponent_C"))
    (if (`KismetSystemLibrary.IsValid` _returnvalue)
      (`/Game/Core/Blueprints/Components/BP_KeypadButtonComponent.SetKeypad` _returnvalue self))))

(fn `AddDigit`
  (params (NewDigit :type "Integer (by ref)"))
  (`self.ResetSystem`)
  (if (not (== (`KismetArrayLibrary.Array_Length` (`self.PasswrdArray`)) (`self.MaxDigit`)))
    (`KismetArrayLibrary.Array_Add` (`self.PasswrdArray`) (`local.NewDigit`))
    (`self.UpdateText`)))

(fn `Correct Password`
  (`GameplayStatics.PlaySound2D` "/Engine/VREditor/Sounds/UI/Camera_Shutter.Camera_Shutter" 1.0 1.0 0.0 null null)
  (`MaterialInstanceDynamic.SetScalarParameterValue` (`self.RedLightMaterial`) "EmissiveStrength" 1.0)
  (`MaterialInstanceDynamic.SetScalarParameterValue` (`self.GreenLightMaterial`) "EmissiveStrength" 50.0)
  (`TextRenderComponent.SetTextRenderColor` (`self.PasswordText`) (`KismetMathLibrary.LinearColor_ToRGBE` (struct :`R` 0.038153 :`G` 1.0 :`A` 1.0)))
  (`/Game/Core/Blueprints/Actors/InteractableActors/BP_DoorSwtich.SwitchActivated` (`self.DoorActor`))
  (for _array_element (`self.GetKeypadButtonArray`)
    (bind _returnvalue (`self.GetComponentByClass` (`ChildActorComponent.ChildActor` _array_element) "/Game/Core/Blueprints/Components/BP_InteractableComponent.BP_InteractableComponent_C"))
    (`/Engine/EditorBlueprintResources/StandardMacros.IsValid` _returnvalue
      (:`Is Valid`
        (`/Game/Core/Blueprints/Components/BP_InteractableComponent.RemoveComponent` _returnvalue)))))

(fn `PasswordCheck`
  (if (== (`KismetStringLibrary.Conv_StringToInt` (`self.Text`)) (`self.Password`))
    (`self.Correct Password`)
    (else
      (`self.WrongPassword`))))

(fn `RemoveDigit`
  (bind _passwrdarray (`self.PasswrdArray`))
  (`self.ResetSystem`)
  (if (`KismetArrayLibrary.Array_IsNotEmpty` _passwrdarray)
    (`KismetArrayLibrary.Array_Remove` (`self.PasswrdArray`) (`KismetArrayLibrary.Array_LastIndex` _passwrdarray))
    (`self.UpdateText`)))

(fn `ResetSystem`
  (`TextRenderComponent.SetTextRenderColor` (`self.PasswordText`) (`KismetMathLibrary.LinearColor_ToRGBE` (struct :`R` 1.0 :`G` 1.0 :`B` 1.0 :`A` 1.0)))
  (`MaterialInstanceDynamic.SetScalarParameterValue` (`self.RedLightMaterial`) "EmissiveStrength" 1.0))

(fn `UpdateText`
  (bind _passwordstringarray (`self.PasswordStringArray`))
  (`KismetArrayLibrary.Array_Clear` (`self.PasswordStringArray`))
  (for _array_element (`self.PasswrdArray`)
    (`KismetArrayLibrary.Array_Add` _passwordstringarray (`KismetStringLibrary.Conv_IntToString` _array_element)))
  (bind _output_get (set `self.Text` (`KismetStringLibrary.Replace` (`BlueprintPathsLibrary.Combine` _passwordstringarray) "/")))
  (`TextRenderComponent.K2_SetText` (`self.PasswordText`) (`KismetTextLibrary.Conv_StringToText` _output_get)))

(fn `UserConstructionScript`
  (`|ExecutionSequence`
    (:`then_0`
      (bind _returnvalue (`PrimitiveComponent.CreateDynamicMaterialInstance` (`self.S_GreenLight`) 0 "/Game/Core/Materials/MI_GreenLight.MI_GreenLight" "None"))
      (bind _output_get (set `self.GreenLightMaterial` _returnvalue))
      (`MaterialInstanceDynamic.SetScalarParameterValue` _output_get "EmissiveStrength" 1.0))
    (:`then_1`
      (bind _returnvalue_2 (`PrimitiveComponent.CreateDynamicMaterialInstance` (`self.S_RedLight`) 0 "/Game/Core/Materials/MI_RedLight.MI_RedLight" "None"))
      (bind _output_get_2 (set `self.RedLightMaterial` _returnvalue_2))
      (`MaterialInstanceDynamic.SetScalarParameterValue` _output_get_2 "EmissiveStrength" 1.0))))

(fn `WrongPassword`
  (`GameplayStatics.PlaySound2D` "/Engine/EditorSounds/Notifications/CompileFailed.CompileFailed" 1.0 1.0 0.0 null null)
  (`MaterialInstanceDynamic.SetScalarParameterValue` (`self.RedLightMaterial`) "EmissiveStrength" 50.0)
  (`TextRenderComponent.SetTextRenderColor` (`self.PasswordText`) (`KismetMathLibrary.LinearColor_ToRGBE` (struct :`R` 1.0 :`A` 1.0)))
  (`KismetSystemLibrary.PrintString` "The try again the password incorrect"))