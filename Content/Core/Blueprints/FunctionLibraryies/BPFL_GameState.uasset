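; Blueprint function library that switches the game between UI and gameplay states for the first local player.
; SetUIMode pauses the game, sets UI-only input and shows the mouse cursor.
; SetGameplayMode reverses this by unpausing, restoring game-only input without flushing it and hiding the cursor.
; A Game-and-UI input node in SetUIMode is left disconnected.
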(fn `SetGameplayMode`
  (params (__WorldContext :type "Object Object Reference"))
  (`GameplayStatics.SetGamePaused` null)
  (`WidgetBlueprintLibrary.SetInputMode_GameOnly` (`GameplayStatics.GetPlayerController` null))
  (set `PlayerController.bShowMouseCursor` false (`GameplayStatics.GetPlayerController` null)))

(fn `SetUIMode`
  (`GameplayStatics.SetGamePaused` null true)
  (`WidgetBlueprintLibrary.SetInputMode_UIOnlyEx` (`GameplayStatics.GetPlayerController` null) null)
  (set `PlayerController.bShowMouseCursor` true (`GameplayStatics.GetPlayerController` null)))