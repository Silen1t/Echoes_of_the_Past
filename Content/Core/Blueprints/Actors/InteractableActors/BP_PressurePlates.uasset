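; Pressure plate actor that activates a linked door actor while something stands on it and deactivates it on exit.
; Capsule overlap calls the door's switch functions, plays open or close sounds, and plays or reverses a timeline that offsets the plate mesh along relative Z.
; A flag and stored actor reference let only the first overlapping actor trigger and release it, ignoring others meanwhile.
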(event `self.ReceiveBeginPlay`
  (set `self.StartLocation` (`SceneComponent.RelativeLocation` (`self.S_PressurePlates`))))

(event `self.Capsule.OnComponentBeginOverlap`
  (params (OverlappedComponent :type "PrimitiveComponent Object Reference") (OtherActor :type "Actor Object Reference") (OtherComp :type "PrimitiveComponent Object Reference") (OtherBodyIndex :type Integer) (bFromSweep :type Boolean) (SweepResult :type "HitResult Structure (by ref)"))
  (bind (_startlocation_x _startlocation_y _startlocation_z) (`KismetMathLibrary.BreakVector` (`self.StartLocation`)))
  (if (`self.CanOverlap`)
    (set `self.LastOverlappedActor` OtherActor)
    (set `self.CanOverlap` false)
    (`KismetSystemLibrary.PrintString` "Hello" true true (struct :`R` 1.0 :`G` 0.141643 :`A` 1.0))
    (`/Game/Core/Blueprints/Actors/InteractableActors/BP_DoorSwtich.SwitchActivated` (`self.DoorActor`))
    (`GameplayStatics.PlaySoundAtLocation` "/Engine/VREditor/Sounds/UI/Dockable_Window_Open.Dockable_Window_Open" (`self.StartLocation`) (struct) 1.0 1.0 0.0 null null null null)
    (bind (_direction _alpha) (`Timeline|TM_PressurePlates` :!label _label)
      (:`Update`
        (`SceneComponent.K2_SetRelativeLocation` (`self.S_PressurePlates`) (`KismetMathLibrary.VLerp` (`self.StartLocation`) (`KismetMathLibrary.MakeVector` _startlocation_x _startlocation_y (+ _startlocation_z (`self.EndLocation`))) _alpha) false false)))))

(event `self.Capsule.OnComponentEndOverlap`
  (params (OverlappedComponent :type "PrimitiveComponent Object Reference") (OtherActor :type "Actor Object Reference") (OtherComp :type "PrimitiveComponent Object Reference") (OtherBodyIndex :type Integer))
  (if (and (== OtherActor (`self.LastOverlappedActor`)) (not (`self.CanOverlap`)))
    (set `self.CanOverlap` true)
    (`KismetSystemLibrary.PrintString` "Hello")
    (`/Game/Core/Blueprints/Actors/InteractableActors/BP_DoorSwtich.SwitchDeactivated` (`self.DoorActor`))
    (`GameplayStatics.PlaySoundAtLocation` "/Engine/VREditor/Sounds/UI/Dockable_Window_Close.Dockable_Window_Close" (`self.StartLocation`) (struct) 1.0 1.0 0.0 null null null null)
    (goto _label :!via `Reverse`)))

(fn `UserConstructionScript`)