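; Actor component that turns its owner into a keypad button, either a digit key or a non-digit key.
; On BeginPlay it binds to the owner's interactable component, provided an ActorSequenceComponent is also present.
; Interaction is ignored while the press sequence plays; otherwise it plays a beep and the sequence at a configurable rate.
; Only digit buttons then pass their digit to the linked keypad actor.
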(event `self.ReceiveBeginPlay`
  (if (`self.IsButtonDigit`)
    (`/Engine/EditorBlueprintResources/StandardMacros.IsValid` (`Actor.GetComponentByClass` (`self.GetOwner`) "/Game/Core/Blueprints/Components/BP_InteractableComponent.BP_InteractableComponent_C")
      (:`Is Valid`
        (`/Engine/EditorBlueprintResources/StandardMacros.IsValid` (`Actor.GetComponentByClass` (`self.GetOwner`) "/Script/ActorSequence.ActorSequenceComponent")
          (:`Is Valid`
            (add `/Game/Core/Blueprints/Components/BP_InteractableComponent.OnObjectInteract` (`Actor.GetComponentByClass` (`self.GetOwner`) "/Game/Core/Blueprints/Components/BP_InteractableComponent.BP_InteractableComponent_C") (delegate `OnObjectInteract_Event`))))))
    (else
      (`/Engine/EditorBlueprintResources/StandardMacros.IsValid` (`Actor.GetComponentByClass` (`self.GetOwner`) "/Game/Core/Blueprints/Components/BP_InteractableComponent.BP_InteractableComponent_C")
        (:`Is Valid`
          (`/Engine/EditorBlueprintResources/StandardMacros.IsValid` (`Actor.GetComponentByClass` (`self.GetOwner`) "/Script/ActorSequence.ActorSequenceComponent")
            (:`Is Valid`
              (add `/Game/Core/Blueprints/Components/BP_InteractableComponent.OnObjectInteract` (`Actor.GetComponentByClass` (`self.GetOwner`) "/Game/Core/Blueprints/Components/BP_InteractableComponent.BP_InteractableComponent_C") (delegate `OnObjectInteract_Event1`)))))))))

(event `OnObjectInteract_Event`
  (params (Player :type "/Game/Core/Blueprints/Characters/FirstPerson/BP_FirstPersonCharacter Object Reference"))
  (bind _returnvalue (`Actor.GetComponentByClass` (`self.GetOwner`) "/Script/ActorSequence.ActorSequenceComponent"))
  (if (not (`MovieSceneSequencePlayer.IsPlaying` (`ActorSequenceComponent.SequencePlayer` _returnvalue)))
    (`GameplayStatics.PlaySound2D` "/UINavigation/Audio/Beep_2_Cue.Beep_2_Cue" 1.0 1.0 0.0 null null)
    (`MovieSceneSequencePlayer.SetPlayRate` (`ActorSequenceComponent.SequencePlayer` _returnvalue) (`self.GetPlayRate`))
    (`ActorSequenceComponent.PlaySequence` _returnvalue)
    (`/Game/Core/Blueprints/Actors/InteractableActors/BP_Keypad.AddDigit` (`self.KeypadActor`) (`self.Digit`))))

(event `OnObjectInteract_Event1`
  (params (Player :type "/Game/Core/Blueprints/Characters/FirstPerson/BP_FirstPersonCharacter Object Reference"))
  (bind _returnvalue (`Actor.GetComponentByClass` (`self.GetOwner`) "/Script/ActorSequence.ActorSequenceComponent"))
  (if (not (`MovieSceneSequencePlayer.IsPlaying` (`ActorSequenceComponent.SequencePlayer` _returnvalue)))
    (`GameplayStatics.PlaySound2D` "/UINavigation/Audio/Beep_2_Cue.Beep_2_Cue" 1.0 1.0 0.0 null null)
    (`MovieSceneSequencePlayer.SetPlayRate` (`ActorSequenceComponent.SequencePlayer` _returnvalue) (`self.GetPlayRate`))
    (`ActorSequenceComponent.PlaySequence` _returnvalue)))

(fn `GetDigit`
  (returns (Digit :type Integer))
  (return (`self.Digit`)))

(fn `GetKeypad`
  (returns (KeypadActor :type "/Game/Core/Blueprints/Actors/InteractableActors/BP_Keypad Object Reference"))
  (return (`self.KeypadActor`)))

(fn `GetPlayRate`
  (returns (PlayRate :type "Float (double-precision)"))
  (return (`self.PlayRate`)))

(fn `SetKeypad`
  (params (KeypadActor :type "/Game/Core/Blueprints/Actors/InteractableActors/BP_Keypad Object Reference"))
  (set `self.KeypadActor` KeypadActor))